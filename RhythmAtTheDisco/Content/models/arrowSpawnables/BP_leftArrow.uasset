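; BP_leftArrow is an arrow actor that travels along its own Path spline and destroys itself at the end.
; Each Tick advances Distance by Speed scaled by delta time, then moves the Sphere component to the spline's local location and rotation at that distance.
; Once Distance exceeds the spline length, the actor is destroyed.
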(event `self.ReceiveTick`
  (params (DeltaSeconds :type "Float (single-precision)"))
  (bind _returnvalue (`SplineComponent.GetTransformAtDistanceAlongSpline` (`self.path`) (`self.distance`) "Local" false))
  (set `self.distance` (+ (* DeltaSeconds (`self.speed`)) (`self.distance`)))
  (`SceneComponent.K2_SetRelativeTransform` (`self.Sphere`) (`KismetMathLibrary.MakeTransform` (.location _returnvalue) (`KismetMathLibrary.MakeRotator` (.roll (.rotation _returnvalue)) (.pitch (.rotation _returnvalue)) (.yaw (.rotation _returnvalue)))) false false)
  (if (> (`self.distance`) (`SplineComponent.GetSplineLength` (`self.path`)))
    (`self.K2_DestroyActor`)))

(fn `UserConstructionScript`)